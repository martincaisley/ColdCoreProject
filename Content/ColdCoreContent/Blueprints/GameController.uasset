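; Player controller for an RTS-style game, handling unit and building selection, move orders and camera control.
; Left mouse starts and stops HUD selection, clearing units when nothing is under the cursor on the selection trace channel.
; Right-click on open ground writes the cursor hit to each selected unit's blackboard TargetLocation, leaving movement to AI.
; F moves the ColdCoreCamera to the first selected unit, and the wheel zooms via spring arm length.
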(event `InputAction|FocusCamera`
  (params (Key :type "Key Structure"))
  ;[1 1 1] Focuses the camera on the first selected unit when the "F" key is pressed
  (:`Pressed`
    (`self.SetCameraLocation` (`self.K2_GetActorLocation` (`|GetArrayItem` (`self.UnitSelection`))))))

(event `self.ReceiveBeginPlay`
  (`WidgetBlueprintLibrary.SetInputMode_GameAndUIEx` self null "LockAlways" false)
  (bind _ascold_core_camera (cast `/Game/ColdCoreContent/Blueprints/ColdCoreCamera` (`self.GetViewTarget`)))
  (set `self.ColdCoreCamera` _ascold_core_camera))

(event `SetCameraLocation`
  (params (location :type "Vector Structure"))
  (bind _defaultsceneroot (`/Game/ColdCoreContent/Blueprints/ColdCoreCamera.DefaultSceneRoot` (`self.ColdCoreCamera`)))
  (`KismetSystemLibrary.MoveComponentTo` _defaultsceneroot location (`SceneComponent.K2_GetComponentRotation` _defaultsceneroot)))

(event `InputAxisKey|MouseWheelAxis`
  (params (AxisValue :type "Float (single-precision)"))
  (if (`self.IsMouseEnabled`)
    (bind _output_get (set `self.ZoomLevel` (`KismetMathLibrary.FClamp` (+ (`self.ZoomLevel`) (* AxisValue -1.0)) 0.0 10.0)))
    (set `SpringArmComponent.TargetArmLength` (+ (* _output_get 200.0) 1000.0) (`/Game/ColdCoreContent/Blueprints/ColdCoreCamera.SpringArm` (`self.ColdCoreCamera`)))))

(event `Key|LeftMouseButton`
  (params (Key :type "Key Structure"))
  (bind _returnvalue (`self.GetHUD`))
  (:`Pressed`
    (message `/Game/ColdCoreContent/Blueprints/SelectionInterface.StartSelection` _returnvalue)
    (if (not (`.ReturnValue` (`self.GetHitResultUnderCursorByChannel` "TraceTypeQuery3")))
      (`self.ClearUnitSelection`)))
  (:`Released`
    (message `/Game/ColdCoreContent/Blueprints/SelectionInterface.StopSelection` _returnvalue)))

(event `Key|RightMouseButton`
  (params (Key :type "Key Structure"))
  (:`Pressed`
    ;[1 1 1] Checks if any actors are under the selection
    (if (not (`.ReturnValue` (`self.GetHitResultUnderCursorByChannel` "TraceTypeQuery3")))
      (for _array_element (`self.UnitSelection`)
        (`BlackboardComponent.SetValueAsVector` (`AIBlueprintHelperLibrary.GetBlackboard` _array_element) "TargetLocation" (`.Location` (`GameplayStatics.BreakHitResult` (`self.GetHitResultUnderCursorByChannel` "TraceTypeQuery1"))))))))

(fn `Add Unit to Selection`
  (params (UnitBase :type "/Game/ColdCoreContent/Units/UnitBase Object Reference"))
  (`KismetArrayLibrary.Array_AddUnique` (`self.UnitSelection`) UnitBase)
  (`/Game/ColdCoreContent/Units/UnitBase.IsSelected` UnitBase true))

(fn `AddBuildingToSelection`
  (params (`Building Base` :type "/Game/ColdCoreContent/Units/UBuildBase Object Reference"))
  (`KismetArrayLibrary.Array_AddUnique` (`self.BuildingSelection`) `Building Base`)
  (`/Game/ColdCoreContent/Units/UBuildBase.IsSelected` `Building Base` true))

(fn `ClearUnitSelection`
  (for _array_element (`self.UnitSelection`)
    (`/Game/ColdCoreContent/Units/UnitBase.IsSelected` _array_element false))
  (`KismetArrayLibrary.Array_Clear` (`self.UnitSelection`))
  (set `self.IsMouseEnabled` true))

(fn `RemoveBuildingFromSelection`
  (params (`Building Base` :type "/Game/ColdCoreContent/Units/UBuildBase Object Reference"))
  (`KismetArrayLibrary.Array_RemoveItem` (`self.BuildingSelection`) `Building Base`)
  (`/Game/ColdCoreContent/Units/UBuildBase.IsSelected` `Building Base` false))

(fn `RemoveUnitFromSelection`
  (params (UnitBase :type "/Game/ColdCoreContent/Units/UnitBase Object Reference"))
  (`KismetArrayLibrary.Array_RemoveItem` (`self.UnitSelection`) UnitBase)
  (`/Game/ColdCoreContent/Units/UnitBase.IsSelected` UnitBase false))

(fn `UserConstructionScript`)