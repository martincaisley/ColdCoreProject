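; ColdCoreHud is a HUD Blueprint that provides drag-box (marquee) selection of UnitBase actors.
; StartSelection records the viewport-scaled mouse position as one corner, and DrawHUD updates the opposite corner while drawing.
; Beyond a minimum drag distance, DrawHUD draws a translucent red rectangle and gathers the units inside it.
; StopSelection replaces the GameController's unit selection with those units, only if a marquee was formed.
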(event `/Game/ColdCoreContent/Blueprints/SelectionInterface.StartSelection`
  (bind _returnvalue (`WidgetLayoutLibrary.GetMousePositionOnViewport`))
  (bind (_returnvalue_x _returnvalue_y) (`KismetMathLibrary.BreakVector2D` (* _returnvalue (`WidgetLayoutLibrary.GetViewportScale`))))
  (set `self.PointA` (`KismetMathLibrary.MakeVector2D` _returnvalue_x _returnvalue_y))
  (set `self.IsDrawing` true))

(event `self.ReceiveBeginPlay`
  (bind _asgame_controller (cast `/Game/ColdCoreContent/Blueprints/GameController` (`GameplayStatics.GetPlayerController` 0)))
  (set `self.As Game Controller` _asgame_controller))

(event `/Game/ColdCoreContent/Blueprints/SelectionInterface.StopSelection`
  (set `self.IsDrawing` false)
  (if (`self.IsMarqee`)
    (`/Game/ColdCoreContent/Blueprints/GameController.ClearUnitSelection` (`self.As Game Controller`))
    (for _array_element (`self.SelectionOfActors`)
      (bind _asunit_base (cast `/Game/ColdCoreContent/Units/UnitBase` _array_element))
      (`/Game/ColdCoreContent/Blueprints/GameController.Add Unit to Selection` (`self.As Game Controller`) _asunit_base))
    (set `self.IsMarqee` false)))

(event `self.ReceiveDrawHUD`
  (params (SizeX :type Integer) (SizeY :type Integer))
  (bind (_pointa_x _pointa_y) (`KismetMathLibrary.BreakVector2D` (`self.PointA`)))
  (bind (_pointb_x _pointb_y) (`KismetMathLibrary.BreakVector2D` (`self.PointB`)))
  (if (`self.IsDrawing`)
    (bind _returnvalue (`WidgetLayoutLibrary.GetMousePositionOnViewport`))
    (bind (_returnvalue_x _returnvalue_y) (`KismetMathLibrary.BreakVector2D` (* _returnvalue (`WidgetLayoutLibrary.GetViewportScale`))))
    (set `self.PointB` (`KismetMathLibrary.MakeVector2D` _returnvalue_x _returnvalue_y))
    (if (> (`KismetMathLibrary.VSize2D` (- (`self.PointA`) (`self.PointB`))) 200.0)
      (`self.DrawRect` (struct :`R` 1.0 :`A` 0.5) _pointa_x _pointa_y (- _pointb_x _pointa_x) (- _pointb_y _pointa_y))
      (set `self.IsMarqee` true)
      (set `self.SelectionOfActors` (`self.GetActorsInSelectionRectangle` "/Game/ColdCoreContent/Units/UnitBase.UnitBase_C" (`self.PointA`) (`self.PointB`)))
      ;[1 1 1] Get amount of selected units
      (set `self.NumberOfSelected` (`KismetArrayLibrary.Array_Length` (`self.SelectionOfActors`))))))

(fn `UserConstructionScript`)